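; BP_AI_Tank is an AI tank Blueprint that handles movement and tracks whether the tank is able to shoot.
; DrivetoLocation and PursueActor share one AI MoveTo node that drives toward a target location or actor and accepts partial paths.
; StopMovement halts the AIFloatingMovement component.
; Overlaps on the Frontal component clear CanShoot on begin and restore it on end; no firing logic appears here.
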(event OnComponentBeginOverlap(Frontal)
  (params (OverlappedComponent :type Primitive%20Component%20Object%20Reference) (OtherActor :type Actor%20Object%20Reference) (OtherComp :type Primitive%20Component%20Object%20Reference) (OtherBodyIndex :type Integer) (bFromSweep :type Boolean) (SweepResult :type Hit%20Result%20Structure%20%28by%20ref%29))
  (Variables|Default|SetCanShoot false))

(event OnComponentEndOverlap(Frontal)
  (params (OverlappedComponent :type Primitive%20Component%20Object%20Reference) (OtherActor :type Actor%20Object%20Reference) (OtherComp :type Primitive%20Component%20Object%20Reference) (OtherBodyIndex :type Integer))
  (Variables|Default|SetCanShoot true))

(event EventBeginPlay
  (|CallParentFunction) ; This node is disabled and will not be called.\nDrag off pins to build functionality.
)

(event EventDrivetoLocation
  (params (target :type Vector :default "0, 0, 0"))
  ;[1 1 1] AI Movement
  (AI|AIMoveTo (AI|GetAIController self) target (stale EventPursueActor target) -1.0 "Disable" "Enable" true true))

(event EventPursueActor
  (params (target :type Actor%20Object%20Reference))
  ;[1 1 1] AI Movement
  (AI|AIMoveTo (AI|GetAIController self) (stale EventDrivetoLocation target) target -1.0 "Disable" "Enable" true true))

(event Collision|EventActorBeginOverlap
  (params (OtherActor :type Actor%20Object%20Reference)))

(event EventTick
  (params (DeltaSeconds :type Float%20%28single-precision%29)))

(event EventStopMovement
  ;[1 1 1] AI Movement
  (Class|NavMovementComponent|StopActiveMovement (Variables|Default|GetAIFloatingMovement)))

(fn ConstructionScript
  (|CallParentFunction))