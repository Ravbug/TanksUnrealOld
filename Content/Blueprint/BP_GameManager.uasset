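; Game manager for a round-based tank game that spawns colored tanks, shows round messages and toggles pause on input.
; SpawnTank overrides the parent, spawning a BP_Tank and tinting chassis, turret and both tracks through dynamic material instances.
; RoundStarting and RoundWon reuse one HUD widget to show the round number or winner and scoreboard, then dismiss it after a short delay.
; The camera look-at logic is disconnected.
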(event EventBeginPlay
  (bind _returnvalue (UserInterface|CreateWidget "/Game/Blueprint/HUD.HUD_C"))
  (Variables|Default|SetHUD _returnvalue))

(event Collision|EventActorBeginOverlap
  (params (OtherActor :type Actor%20Object%20Reference)))

(event EventTick
  (params (DeltaSeconds :type Float%20%28single-precision%29))
  ;[1 1 1] Face camera towards base (broken)
)

(event EventRoundStarting
  (params (round :type Integer))
  (bind _hud (Variables|Default|GetHUD))
  (bind _roundtext (Variables|/Game/Blueprint/HUD.HUD_C|GetRoundText _hud))
  ;[1 1 1] Show the HUD with just the round number
  (UserInterface|Viewport|AddtoViewport _hud 0)
  (Widget|SetVisibility _roundtext "Visible")
  (Rendering|Components|TextRender|SetText _roundtext (Utilities|Text|ToText(String) (Utilities|String|Append "Round  " (Utilities|String|ToString(Integer) round))))
  (Widget|SetVisibility (Variables|/Game/Blueprint/HUD.HUD_C|GetWinnerText _hud) "Hidden")
  (Widget|SetVisibility (Variables|/Game/Blueprint/HUD.HUD_C|GetScoreboardText _hud) "Hidden")
  (Utilities|FlowControl|Delay 3.0)
  (Class|GameManager|DismissHUD))

(event EventDismissHUD
  ;[1 1 1] Dismiss the HUD
  (Widget|RemovefromParent (Variables|Default|GetHUD)))

(event EventRoundWon
  (params (text :type String) (scoreboard :type String))
  (bind _hud (Variables|Default|GetHUD))
  (bind _scoreboardtext (Variables|/Game/Blueprint/HUD.HUD_C|GetScoreboardText _hud))
  (bind _winnertext (Variables|/Game/Blueprint/HUD.HUD_C|GetWinnerText _hud))
  ;[1 1 1] Show the HUD when the round is won
  (UserInterface|Viewport|AddtoViewport _hud 0)
  (Widget|SetVisibility (Variables|/Game/Blueprint/HUD.HUD_C|GetRoundText _hud) "Hidden")
  (Widget|SetVisibility _winnertext "Visible")
  (Widget|SetVisibility _scoreboardtext "Visible")
  (Rendering|Components|TextRender|SetText _winnertext (Utilities|Text|ToText(String) text))
  (Rendering|Components|TextRender|SetText _scoreboardtext (Utilities|Text|ToText(String) scoreboard))
  (Utilities|FlowControl|Delay 3.0)
  (Class|GameManager|DismissHUD))

(event Input|ActionEvents|InputActionPause
  (params (Key :type Key%20Structure))
  (:Pressed
    (bind _output_get (Variables|Default|SetPaused (not (Variables|Default|GetPaused))))
    (Game|SetGamePaused _output_get)))

(fn ConstructionScript)

(fn SpawnTank
  (params (color :type Color%20Structure) (pos :type Transform))
  (bind _returnvalue (Math|Conversions|ToLinearColor(Color) color))
  (|CallParentFunction color pos)
  (bind _returnvalue_2 (Game|SpawnActorfromClass "/Game/Blueprint/BP_Tank.BP_Tank_C" pos "Undefined" 0 0))
  (bind _returnvalue_3 (Rendering|Material|CreateDynamicMaterialInstance (Variables|/Game/Blueprint/BP_Tank.BP_Tank_C|GetTank_TankChassis _returnvalue_2) 0 "/Game/Material/TankColour.TankColour" "None" :!class /Script/Engine.PrimitiveComponent))
  (Rendering|Material|SetVectorParameterValue _returnvalue_3 "TankColor" _returnvalue :!class /Script/Engine.MaterialInstanceDynamic)
  (bind _returnvalue_4 (Rendering|Material|CreateDynamicMaterialInstance (Variables|/Game/Blueprint/BP_Tank.BP_Tank_C|GetTank_TankTurret _returnvalue_2) 0 "/Game/Material/TankColour.TankColour" "None" :!class /Script/Engine.PrimitiveComponent))
  (Rendering|Material|SetVectorParameterValue _returnvalue_4 "TankColor" _returnvalue :!class /Script/Engine.MaterialInstanceDynamic)
  (bind _returnvalue_5 (Rendering|Material|CreateDynamicMaterialInstance (Variables|/Game/Blueprint/BP_Tank.BP_Tank_C|GetTank_TankTracksLeft _returnvalue_2) 0 "/Game/Material/TankColour.TankColour" "None" :!class /Script/Engine.PrimitiveComponent))
  (Rendering|Material|SetVectorParameterValue _returnvalue_5 "TankColor" _returnvalue :!class /Script/Engine.MaterialInstanceDynamic)
  (bind _returnvalue_6 (Rendering|Material|CreateDynamicMaterialInstance (Variables|/Game/Blueprint/BP_Tank.BP_Tank_C|GetTank_TankTracksRight _returnvalue_2) 0 "/Game/Material/TankColour.TankColour" "None" :!class /Script/Engine.PrimitiveComponent))
  (Rendering|Material|SetVectorParameterValue _returnvalue_6 "TankColor" _returnvalue :!class /Script/Engine.MaterialInstanceDynamic)
  (return _returnvalue_2))