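; BP_Tank is a tank actor that exposes events for firing, dying and toggling its visibility.
; Fire spawns a Bullet at the BulletSpawn transform, passing Power as its initial velocity.
; Die spawns an Explosion at the chassis and hides the chassis with its children, without destroying the actor.
; SetSelfVisibility shows or hides that same hierarchy; the Blueprint has no active Tick or input logic.
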(event EventBeginPlay)

(event Collision|EventActorBeginOverlap
  (params (OtherActor :type Actor%20Object%20Reference)))

(event EventTick
  (params (DeltaSeconds :type Float%20%28single-precision%29)))

(event EventFire
  (params (power :type Integer))
  ;[1 1 1] Fire bullets with specified strength
  (Game|SpawnActorfromClass "/Game/Blueprint/Bullet.Bullet_C" (Transformation|GetWorldTransform (Variables|Default|GetBulletSpawn)) "Undefined" 0 power 0))

(event EventDie
  ;[1 1 1] On death, spawn an explosion and disable actor
  (Game|SpawnActorfromClass "/Game/Blueprint/Explosion.Explosion_C" (Transformation|GetWorldTransform (Variables|Default|GetTank_TankChassis)) "Undefined" 0 0)
  (Rendering|SetVisibility (Variables|Default|GetTank_TankChassis) false true))

(event EventSetSelfVisibility
  (params (visible :type Boolean))
  ;[1 1 1] Toggle visibility
  (Rendering|SetVisibility (Variables|Default|GetTank_TankChassis) visible true))

(fn ConstructionScript)