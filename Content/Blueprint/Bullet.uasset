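; Bullet is a projectile actor that plays a firing sound on spawn and explodes on impact.
; The construction script sets the ProjectileMovement initial speed from InitialVelocity and gives the actor a short lifespan.
; A Shell component hit spawns an Explosion actor, plays a tank explosion sound and destroys the bullet.
; Both sounds scale their volume with InitialVelocity and randomize pitch for variety.
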(event OnComponentHit(Shell)
  (params (HitComponent :type Primitive%20Component%20Object%20Reference) (OtherActor :type Actor%20Object%20Reference) (OtherComp :type Primitive%20Component%20Object%20Reference) (NormalImpulse :type Vector :default "0, 0, 0") (Hit :type Hit%20Result%20Structure%20%28by%20ref%29))
  ;[1 1 1] When the bullet hits something, spawn an explosion and remove self
  (Game|SpawnActorfromClass "/Game/Blueprint/Explosion.Explosion_C" (Transformation|GetWorldTransform (Variables|Default|GetShell)) "Undefined" 0 3.0 0)
  (Audio|PlaySoundatLocation "/Game/Sound/TankExplosion.TankExplosion" (Transformation|GetActorLocation) "0, 0, 0" (/ (Math|Conversions|ToFloat(Integer) (Variables|Default|GetInitialVelocity)) 3e+01) (Math|Random|RandomFloatinRange 0.5 1.7) 0.0 0 0 0)
  (Actor|DestroyActor))

(event EventBeginPlay
  ;[1 1 1] Play fire sound when actor spawns
  (Audio|PlaySoundatLocation "/Game/Sound/ShotFiring.ShotFiring" (Transformation|GetActorLocation) "0, 0, 0" (/ (Math|Conversions|ToFloat(Integer) (Variables|Default|GetInitialVelocity)) 3e+01) (Math|Random|RandomFloatinRange 0.5 1.7) 0.0 0 0 0))

(event Collision|EventActorBeginOverlap
  (params (OtherActor :type Actor%20Object%20Reference)))

(event EventTick
  (params (DeltaSeconds :type Float%20%28single-precision%29)))

(fn ConstructionScript
  ;[1 1 1] Set the actor max lifespan and initial velocity on spawn
  (Variables|/Script/Engine.ProjectileMovementComponent|SetInitialSpeed (Variables|Default|GetProjectileMovement) (Math|Conversions|ToFloat(Integer) (* (Variables|Default|GetInitialVelocity) 100)))
  (Actor|SetLifeSpan 5.0))